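; BP_Capital is a capital ship target that awards points to the player when its parts are hit.
; Component hit events on the hull base, engines, fans, armor, fins, guns, satellite and generator feed three shared scoring paths, each worth a different amount.
; Each path casts the player pawn to BP_Canon_Barrel and adds to its Points, without checking what struck the component.
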(event OnComponentHit(Fins)
  (params (HitComponent :type Primitive%20Component%20Object%20Reference) (OtherActor :type Actor%20Object%20Reference) (OtherComp :type Primitive%20Component%20Object%20Reference) (NormalImpulse :type Vector :default "0, 0, 0") (Hit :type Hit%20Result%20Structure%20%28by%20ref%29))
  ;[1 1 1] Points
  (bind _asbp_canon_barrel (Utilities|Casting|CastToBP_Canon_Barrel (Game|Player|GetPlayerPawn 0)))
  (Variables|/Game/Canon/BP_Canon_Barrel.BP_Canon_Barrel_C|SetPoints _asbp_canon_barrel (+ (Variables|/Game/Canon/BP_Canon_Barrel.BP_Canon_Barrel_C|GetPoints _asbp_canon_barrel) 50)))

(event OnComponentHit(Fan1)
  (params (HitComponent :type Primitive%20Component%20Object%20Reference) (OtherActor :type Actor%20Object%20Reference) (OtherComp :type Primitive%20Component%20Object%20Reference) (NormalImpulse :type Vector :default "0, 0, 0") (Hit :type Hit%20Result%20Structure%20%28by%20ref%29))
  ;[1 1 1] Points
  (bind _asbp_canon_barrel (Utilities|Casting|CastToBP_Canon_Barrel (Game|Player|GetPlayerPawn 0)))
  (Variables|/Game/Canon/BP_Canon_Barrel.BP_Canon_Barrel_C|SetPoints _asbp_canon_barrel (+ (Variables|/Game/Canon/BP_Canon_Barrel.BP_Canon_Barrel_C|GetPoints _asbp_canon_barrel) 150)))

(event OnComponentHit(CapitalBase)
  (params (HitComponent :type Primitive%20Component%20Object%20Reference) (OtherActor :type Actor%20Object%20Reference) (OtherComp :type Primitive%20Component%20Object%20Reference) (NormalImpulse :type Vector :default "0, 0, 0") (Hit :type Hit%20Result%20Structure%20%28by%20ref%29))
  ;[1 1 1] Points
  (bind _asbp_canon_barrel (Utilities|Casting|CastToBP_Canon_Barrel (Game|Player|GetPlayerPawn 0)))
  (Variables|/Game/Canon/BP_Canon_Barrel.BP_Canon_Barrel_C|SetPoints _asbp_canon_barrel (+ (Variables|/Game/Canon/BP_Canon_Barrel.BP_Canon_Barrel_C|GetPoints _asbp_canon_barrel) 100)))

(event OnComponentHit(Fan2)
  (params (HitComponent :type Primitive%20Component%20Object%20Reference) (OtherActor :type Actor%20Object%20Reference) (OtherComp :type Primitive%20Component%20Object%20Reference) (NormalImpulse :type Vector :default "0, 0, 0") (Hit :type Hit%20Result%20Structure%20%28by%20ref%29))
  ;[1 1 1] Points
  (bind _asbp_canon_barrel (Utilities|Casting|CastToBP_Canon_Barrel (Game|Player|GetPlayerPawn 0)))
  (Variables|/Game/Canon/BP_Canon_Barrel.BP_Canon_Barrel_C|SetPoints _asbp_canon_barrel (+ (Variables|/Game/Canon/BP_Canon_Barrel.BP_Canon_Barrel_C|GetPoints _asbp_canon_barrel) 150)))

(event OnComponentHit(Fan3)
  (params (HitComponent :type Primitive%20Component%20Object%20Reference) (OtherActor :type Actor%20Object%20Reference) (OtherComp :type Primitive%20Component%20Object%20Reference) (NormalImpulse :type Vector :default "0, 0, 0") (Hit :type Hit%20Result%20Structure%20%28by%20ref%29))
  ;[1 1 1] Points
  (bind _asbp_canon_barrel (Utilities|Casting|CastToBP_Canon_Barrel (Game|Player|GetPlayerPawn 0)))
  (Variables|/Game/Canon/BP_Canon_Barrel.BP_Canon_Barrel_C|SetPoints _asbp_canon_barrel (+ (Variables|/Game/Canon/BP_Canon_Barrel.BP_Canon_Barrel_C|GetPoints _asbp_canon_barrel) 50)))

(event OnComponentHit(Guns)
  (params (HitComponent :type Primitive%20Component%20Object%20Reference) (OtherActor :type Actor%20Object%20Reference) (OtherComp :type Primitive%20Component%20Object%20Reference) (NormalImpulse :type Vector :default "0, 0, 0") (Hit :type Hit%20Result%20Structure%20%28by%20ref%29))
  ;[1 1 1] Points
  (bind _asbp_canon_barrel (Utilities|Casting|CastToBP_Canon_Barrel (Game|Player|GetPlayerPawn 0)))
  (Variables|/Game/Canon/BP_Canon_Barrel.BP_Canon_Barrel_C|SetPoints _asbp_canon_barrel (+ (Variables|/Game/Canon/BP_Canon_Barrel.BP_Canon_Barrel_C|GetPoints _asbp_canon_barrel) 150)))

(event OnComponentHit(Generator)
  (params (HitComponent :type Primitive%20Component%20Object%20Reference) (OtherActor :type Actor%20Object%20Reference) (OtherComp :type Primitive%20Component%20Object%20Reference) (NormalImpulse :type Vector :default "0, 0, 0") (Hit :type Hit%20Result%20Structure%20%28by%20ref%29))
  ;[1 1 1] Points
  (bind _asbp_canon_barrel (Utilities|Casting|CastToBP_Canon_Barrel (Game|Player|GetPlayerPawn 0)))
  (Variables|/Game/Canon/BP_Canon_Barrel.BP_Canon_Barrel_C|SetPoints _asbp_canon_barrel (+ (Variables|/Game/Canon/BP_Canon_Barrel.BP_Canon_Barrel_C|GetPoints _asbp_canon_barrel) 150)))

(event OnComponentHit(Armor)
  (params (HitComponent :type Primitive%20Component%20Object%20Reference) (OtherActor :type Actor%20Object%20Reference) (OtherComp :type Primitive%20Component%20Object%20Reference) (NormalImpulse :type Vector :default "0, 0, 0") (Hit :type Hit%20Result%20Structure%20%28by%20ref%29))
  ;[1 1 1] Points
  (bind _asbp_canon_barrel (Utilities|Casting|CastToBP_Canon_Barrel (Game|Player|GetPlayerPawn 0)))
  (Variables|/Game/Canon/BP_Canon_Barrel.BP_Canon_Barrel_C|SetPoints _asbp_canon_barrel (+ (Variables|/Game/Canon/BP_Canon_Barrel.BP_Canon_Barrel_C|GetPoints _asbp_canon_barrel) 50)))

(event OnComponentHit(Engines)
  (params (HitComponent :type Primitive%20Component%20Object%20Reference) (OtherActor :type Actor%20Object%20Reference) (OtherComp :type Primitive%20Component%20Object%20Reference) (NormalImpulse :type Vector :default "0, 0, 0") (Hit :type Hit%20Result%20Structure%20%28by%20ref%29))
  ;[1 1 1] Points
  (bind _asbp_canon_barrel (Utilities|Casting|CastToBP_Canon_Barrel (Game|Player|GetPlayerPawn 0)))
  (Variables|/Game/Canon/BP_Canon_Barrel.BP_Canon_Barrel_C|SetPoints _asbp_canon_barrel (+ (Variables|/Game/Canon/BP_Canon_Barrel.BP_Canon_Barrel_C|GetPoints _asbp_canon_barrel) 100)))

(event OnComponentHit(Sat)
  (params (HitComponent :type Primitive%20Component%20Object%20Reference) (OtherActor :type Actor%20Object%20Reference) (OtherComp :type Primitive%20Component%20Object%20Reference) (NormalImpulse :type Vector :default "0, 0, 0") (Hit :type Hit%20Result%20Structure%20%28by%20ref%29))
  ;[1 1 1] Points
  (bind _asbp_canon_barrel (Utilities|Casting|CastToBP_Canon_Barrel (Game|Player|GetPlayerPawn 0)))
  (Variables|/Game/Canon/BP_Canon_Barrel.BP_Canon_Barrel_C|SetPoints _asbp_canon_barrel (+ (Variables|/Game/Canon/BP_Canon_Barrel.BP_Canon_Barrel_C|GetPoints _asbp_canon_barrel) 150)))

(fn ConstructionScript)