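; BP_Ball is the cannon game's bouncing projectile, with speed tiers set each tick from the player barrel's points.
; Each hit counts a bounce and restarts a countdown; its finish or the third bounce homes the ball to BP_MiddleCollision, turns it red and changes the ring's light.
; Reaching the bounce limit also sets CanPassThrough.
; HomingReturn retargets a random BP_Collision at reduced speed, repeating on overlaps while IsHomingReturn is set.
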(event EventBeginPlay
  ;[1 1 1] MaxBounceSet
  (Variables|Default|SetMaxBounce 3)
  ;[1 1 1] StartHoming
  (Timeline|CountDown Play
    (:Finished
      (CallFunction|HomingMiddle)
      (Rendering|Material|SetVectorParameterValue (Variables|Default|GetReturnBall) "BallLight" "(R=1.000000,G=0.000000,B=0.000000,A=1.000000)" :!class /Script/Engine.MaterialInstanceDynamic)
      (Rendering|Material|SetVectorParameterValue (Variables|Default|GetReturnBallClear) "ColorGlass" "(R=1.000000,G=0.000000,B=0.000000,A=1.000000)" :!class /Script/Engine.MaterialInstanceDynamic)
      (bind _returnvalue (Actor|GetActorOfClass "/Game/LevelParts/BP_BaseRing.BP_BaseRing_C"))
      (Default|ReturnLightChange _returnvalue))))

(event Collision|EventActorBeginOverlap
  (params (OtherActor :type Actor%20Object%20Reference))
  ;[1 1 1] BallHomingReturnMain
  (if (Variables|Default|GetIsHomingReturn)
    (CallFunction|HomingReturn)))

(event EventTick
  (params (DeltaSeconds :type Float%20%28single-precision%29))
  ;[1 1 1] BallSpeed_CanPassCondition
  (if (>= (Variables|Default|GetBounceCount) (Variables|Default|GetMaxBounce))
    (Variables|Default|SetCanPassThrough true)
    (else
      (Variables|Default|SetCanPassThrough false)))
  (bind _asbp_canon_barrel (Utilities|Casting|CastToBP_Canon_Barrel (Game|Player|GetPlayerPawn 0)))
  (switch int (Math|Float|Truncate (* (Variables|/Game/Canon/BP_Canon_Barrel.BP_Canon_Barrel_C|GetPoints _asbp_canon_barrel) 0.001))
    (:Default
      (Variables|Default|SetDificulty%20Speed 2e+03))
    (:0
      (Variables|Default|SetDificulty%20Speed 2e+03))
    (:1
      (Variables|Default|SetDificulty%20Speed 2.25e+03))
    (:2
      (Variables|Default|SetDificulty%20Speed 2.5e+03))
    (:3
      (Variables|Default|SetDificulty%20Speed 2.75e+03))
    (:4
      (Variables|Default|SetDificulty%20Speed 3e+03))
    (:5
      (Variables|Default|SetDificulty%20Speed 3.5e+03))))

(event Collision|EventHit
  (params (MyComp :type Primitive%20Component%20Object%20Reference) (Other :type Actor%20Object%20Reference) (OtherComp :type Primitive%20Component%20Object%20Reference) (bSelfMoved :type Boolean) (HitLocation :type Vector :default "0, 0, 0") (HitNormal :type Vector :default "0, 0, 0") (NormalImpulse :type Vector :default "0, 0, 0") (Hit :type Hit%20Result%20Structure%20%28by%20ref%29))
  ;[1 1 1] StartHoming
  (bind _output_get (Variables|Default|SetBounceCount (+ (stale _output_get) 1)))
  (Variables|/Script/Engine.ProjectileMovementComponent|SetInitialSpeed (Variables|Default|GetProjectileMovement) (Variables|Default|GetDificulty%20Speed))
  (if (>= (Variables|Default|GetBounceCount) (Variables|Default|GetMaxBounce))
    _
    (else
      (Timeline|CountDown PlayFromStart
        (:Finished
          _))))
  (CallFunction|HomingMiddle)
  (Rendering|Material|SetVectorParameterValue (Variables|Default|GetReturnBall) "BallLight" "(R=1.000000,G=0.000000,B=0.000000,A=1.000000)" :!class /Script/Engine.MaterialInstanceDynamic)
  (Rendering|Material|SetVectorParameterValue (Variables|Default|GetReturnBallClear) "ColorGlass" "(R=1.000000,G=0.000000,B=0.000000,A=1.000000)" :!class /Script/Engine.MaterialInstanceDynamic)
  (bind _returnvalue (Actor|GetActorOfClass "/Game/LevelParts/BP_BaseRing.BP_BaseRing_C"))
  (Default|ReturnLightChange _returnvalue))

(fn ConstructionScript
  (bind _ball (Variables|Default|GetBall))
  (bind _returnvalue (Rendering|Material|CreateDynamicMaterialInstance _ball 2 0 "None" :!class /Script/Engine.PrimitiveComponent))
  (Variables|Default|SetReturnBall _returnvalue)
  (bind _returnvalue_2 (Rendering|Material|CreateDynamicMaterialInstance _ball 1 0 "None" :!class /Script/Engine.PrimitiveComponent))
  (Variables|Default|SetReturnBallClear _returnvalue_2))

(fn HomingMiddle
  (bind _projectilemovement (Variables|Default|GetProjectileMovement))
  ;[1 1 1] Targeting Middle Location
  (Physics|SetSimulatePhysics (Variables|Default|GetBall) false)
  (Variables|/Script/Engine.ProjectileMovementComponent|SetbIsHomingProjectile _projectilemovement true)
  (Variables|/Script/Engine.ProjectileMovementComponent|SetMaxSpeed _projectilemovement (Variables|Default|GetDificulty%20Speed))
  (bind _returnvalue (Actor|GetActorOfClass "/Game/LevelParts/BP_MiddleCollision.BP_MiddleCollision_C"))
  (Variables|/Script/Engine.ProjectileMovementComponent|SetHomingTargetComponent _projectilemovement (Variables|/Game/LevelParts/BP_MiddleCollision.BP_MiddleCollision_C|GetMidLoc _returnvalue))
  (Variables|/Script/Engine.ProjectileMovementComponent|SetHomingAccelerationMagnitude _projectilemovement 1.5e+04)
  (Variables|Default|SetIsHomingMiddle true))

(fn HomingReturn
  (bind _projectilemovement (Variables|Default|GetProjectileMovement))
  (Variables|Default|SetIsHomingReturn true)
  (Physics|SetSimulatePhysics (Variables|Default|GetBall) false)
  (Variables|/Script/Engine.ProjectileMovementComponent|SetbIsHomingProjectile _projectilemovement true)
  (Variables|/Script/Engine.ProjectileMovementComponent|SetMaxSpeed _projectilemovement (- (Variables|Default|GetDificulty%20Speed) 3e+02))
  (bind _outactors (Actor|GetAllActorsOfClass "/Game/LevelParts/BP_Collision.BP_Collision_C"))
  (Variables|/Script/Engine.ProjectileMovementComponent|SetHomingTargetComponent _projectilemovement (Variables|/Game/LevelParts/BP_Collision.BP_Collision_C|GetColLoc (Utilities|Array|Get(acopy) _outactors (Math|Random|RandomIntegerinRange 0 2))))
  (Variables|/Script/Engine.ProjectileMovementComponent|SetHomingAccelerationMagnitude _projectilemovement 8e+03))

(fn BallMatChange
  (Rendering|Material|SetVectorParameterValue (Variables|Default|GetReturnBall) "None" "(R=1.000000,G=0.000000,B=0.000000,A=1.000000)" :!class /Script/Engine.MaterialInstanceDynamic))