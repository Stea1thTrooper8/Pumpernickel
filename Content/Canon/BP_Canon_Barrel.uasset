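; Player-controlled cannon that slides left and right, fires balls one at a time and holds the station's HP and score.
; Mouse axes move a clamped aim target; look-at rotations turn the barrel, and the camera-to-target rotation sets the ball's launch direction.
; A catch collider destroys deletable balls, re-enabling fire and resetting the ring light.
; Tick spawns fixed-position damage effects as HP drops and saves the high score to the game instance below one HP.
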(event OnComponentBeginOverlap(BallCatchCol)
  (params (OverlappedComponent :type Primitive%20Component%20Object%20Reference) (OtherActor :type Actor%20Object%20Reference) (OtherComp :type Primitive%20Component%20Object%20Reference) (OtherBodyIndex :type Integer) (bFromSweep :type Boolean) (SweepResult :type Hit%20Result%20Structure%20%28by%20ref%29))
  ;[1 1 1] Ball_Catch
  (bind _asbp_ball (Utilities|Casting|CastToBP_Ball OtherActor))
  (if (Variables|/Game/Canon/BP_Ball.BP_Ball_C|GetCanBeDeleted _asbp_ball)
    (Variables|/Game/Canon/BP_Ball.BP_Ball_C|SetCanBeDeleted _asbp_ball false)
    (Variables|/Game/Canon/BP_Ball.BP_Ball_C|SetIsHomingReturn _asbp_ball false)
    (Actor|DestroyActor _asbp_ball)
    (Variables|Default|SetBallCount 0)
    (bind _returnvalue (Actor|GetActorOfClass "/Game/LevelParts/BP_BaseRing.BP_BaseRing_C"))
    (Default|ReturnLightNormal _returnvalue)))

(event EventBeginPlay
  (bind _aim (Variables|Default|GetAim))
  (bind _returnvalue (Transformation|GetWorldLocation _aim))
  ;[1 1 1] Widget_Start
  (bind _returnvalue_2 (UserInterface|CreateWidget "/Game/instance_Interface/BP_GameplayInterface.BP_GameplayInterface_C"))
  (UserInterface|Viewport|AddtoViewport _returnvalue_2 0)
  ;[1 1 1] Set_Vars
  (Variables|Default|SetStationHP 3)
  (Variables|Default|SetPoints 0)
  (Variables|Default|SetAimRelativeLocation (.location (Transformation|GetRelativeTransform (Variables|Default|GetAim))))
  (Variables|Default|SetXAimAxis (- (.x _returnvalue) (.x (stale _output_get))))
  (Variables|Default|SetYAimAxis (- (.z _returnvalue) (.z (stale _output_get))))
  (bind _output_get (Variables|Default|SetAimOriginalLocation (Math|Vector|MakeVector (.x _returnvalue) (.y _returnvalue) (.z _returnvalue))))
  ;[1 1 1] Keep_Cannon_InRange
  (bind _output_get_2 (Variables|Default|SetCanonOriginalLocation (.x (Transformation|GetActorLocation))))
  (bind _output_get_3 (Variables|Default|SetCanonXRange 5e+02)))

(event EventTick
  (params (DeltaSeconds :type Float%20%28single-precision%29))
  ;[1 1 1] Highscore_StationBreaking
  (CallFunction|HighScore)
  (CallFunction|StationBreaking))

(event Input|AxisEvents|InputAxisMouseY
  (params (AxisValue :type Float%20%28single-precision%29))
  (bind _aim (Variables|Default|GetAim))
  (bind _returnvalue (Transformation|GetWorldLocation _aim))
  ;[1 1 1] Aim_Location
  (bind _output_get (Variables|Default|SetYAimAxis (+ (* AxisValue 15.0) (stale _output_get_2))))
  (if (< _output_get 1.4e+03)
    (if (> _output_get -5e+02)
      (bind _output_get_2 (Variables|Default|SetYAimAxis (Variables|Default|GetYAimAxis)))
      ;[1 1 1] Canon_Aiming_Rotation_Tracking
      (Transformation|SetRelativeLocation (Variables|Default|GetAim) (Math|Vector|MakeVector (.x (Variables|Default|GetAimRelativeLocation)) (Variables|Default|GetXAimAxis) (Variables|Default|GetYAimAxis)) true false)
      (Transformation|SetWorldRotation (Variables|Default|GetAim) (Math|Rotator|FindLookatRotation (Transformation|GetWorldLocation (Variables|Default|GetRotationPoint)) _returnvalue) false false)
      (Transformation|SetWorldRotation (Variables|GetMeshComponent) (Math|Rotator|FindLookatRotation (Transformation|GetWorldLocation (Variables|GetMeshComponent)) _returnvalue) false false)
      (Variables|Default|SetAimRot (Math|Rotator|FindLookatRotation (Transformation|GetWorldLocation (Variables|/Script/Engine.CameraActor|GetCameraComponent (Variables|Default|GetCameraLocation))) _returnvalue))
      (else
        (Variables|Default|SetYAimAxis -5e+02)))
    (else
      (Variables|Default|SetYAimAxis 1399.0))))

(event Input|AxisEvents|InputAxisMoveRight
  (params (AxisValue :type Float%20%28single-precision%29))
  (bind _returnvalue (Transformation|GetActorLocation))
  ;[1 1 1] Movement_Left_Right
  (if (Math|Float|InRange(Float) (Math|Float|Absolute(Float) (- (.x (Transformation|GetActorLocation)) (stale EventBeginPlay _output_get_2))) (- (stale EventBeginPlay _output_get_2) (stale EventBeginPlay _output_get_3)) (+ (stale EventBeginPlay _output_get_3) (stale EventBeginPlay _output_get_2)) false false)
    (Pawn|Input|AddMovementInput (Math|Vector|MakeVector (.x (Transformation|GetActorRightVector)) 0.0 0.0) AxisValue true)
    (else
      (Transformation|SetActorLocation (Math|Vector|MakeVector (* (* (.x _returnvalue) -0.002) -499.0) (.y _returnvalue) (.z _returnvalue)) false false))))

(event Input|AxisEvents|InputAxisMouseX
  (params (AxisValue :type Float%20%28single-precision%29))
  (bind _aim (Variables|Default|GetAim))
  (bind _returnvalue (Transformation|GetWorldLocation _aim))
  ;[1 1 1] Aim_Location
  (bind _output_get (Variables|Default|SetXAimAxis (+ (* AxisValue 1e+01) (stale _output_get_2))))
  (if (< _output_get 8e+02)
    (if (> _output_get -8e+02)
      (bind _output_get_2 (Variables|Default|SetXAimAxis (Variables|Default|GetXAimAxis)))
      ;[1 1 1] Canon_Aiming_Rotation_Tracking
      (Transformation|SetRelativeLocation (Variables|Default|GetAim) (Math|Vector|MakeVector (.x (Variables|Default|GetAimRelativeLocation)) (Variables|Default|GetXAimAxis) (Variables|Default|GetYAimAxis)) true false)
      (Transformation|SetWorldRotation (Variables|Default|GetAim) (Math|Rotator|FindLookatRotation (Transformation|GetWorldLocation (Variables|Default|GetRotationPoint)) _returnvalue) false false)
      (Transformation|SetWorldRotation (Variables|GetMeshComponent) (Math|Rotator|FindLookatRotation (Transformation|GetWorldLocation (Variables|GetMeshComponent)) _returnvalue) false false)
      (Variables|Default|SetAimRot (Math|Rotator|FindLookatRotation (Transformation|GetWorldLocation (Variables|/Script/Engine.CameraActor|GetCameraComponent (Variables|Default|GetCameraLocation))) _returnvalue))
      (else
        (Variables|Default|SetXAimAxis -799.0)))
    (else
      (Variables|Default|SetXAimAxis 799.0))))

(event Input|KeyboardEvents|SpaceBar
  (params (Key :type Key%20Structure :default "None"))
  (bind _ballspawn (Variables|Default|GetBallSpawn))
  (bind _returnvalue (Transformation|GetWorldLocation _ballspawn))
  ;[1 1 1] Ball_Spawn
  (:Pressed
    (if (not (== (Variables|Default|GetBallCount) 1))
      (Game|SpawnActorfromClass "/Game/Canon/BP_Ball.BP_Ball_C" (Math|Transform|MakeTransform _returnvalue (Variables|Default|GetAimRot) "3.000000,3.000000,3.000000") "AlwaysSpawn" 0 0)
      (bind _output_get (Variables|Default|SetBallCount (+ (stale _output_get) 1)))
      (Effects|SpawnEmitteratLocation "/Game/ParticleSys/P_ExplosionGun.P_ExplosionGun" _returnvalue "0, 0, 0" "2.000000,2.000000,2.000000"))))

(fn ConstructionScript)

(fn HighScore
  (bind _points (Variables|Default|GetPoints))
  (if (< (Variables|Default|GetStationHP) 1)
    (bind _ascanon_game_instance (Utilities|Casting|CastToCanonGameInstance (Game|GetGameInstance)))
    (if (< (Variables|/Game/instance_Interface/CanonGameInstance.CanonGameInstance_C|GetHighScore _ascanon_game_instance) _points)
      (Variables|/Game/instance_Interface/CanonGameInstance.CanonGameInstance_C|SetHighScore _ascanon_game_instance _points))))

(fn StationBreaking
  (bind _stationhp (Variables|Default|GetStationHP))
  (if (<= _stationhp 2)
    (if (Variables|Default|GetFireSpawned)
      (if (<= _stationhp 1)
        (if (not (Variables|Default|GetSparksSpawned))
          (Effects|SpawnEmitteratLocation "/Game/StarterContent/Particles/P_Explosion.P_Explosion" "865.000000,-115.000000,900.000000" "0, 0, 0" "3.000000,3.000000,3.000000")
          (Effects|SpawnEmitteratLocation "/Game/ParticleSys/P_Sparks.P_Sparks" "865.000000,-115.000000,900.000000" "0, 0, 0" "2.000000,2.000000,2.000000" false)
          (Variables|Default|SetSparksSpawned true)))
      (else
        (Effects|SpawnEmitteratLocation "/Game/StarterContent/Particles/P_Explosion.P_Explosion" "-860.000000,-115.000000,-90.000000" "0, 0, 0" "3.000000,3.000000,3.000000")
        (Effects|SpawnEmitteratLocation "/Game/ParticleSys/P_Fire.P_Fire" "-860.000000,-115.000000,-90.000000" "0, 0, 0" "2.000000,2.000000,2.000000" false)
        (Variables|Default|SetFireSpawned true)))))