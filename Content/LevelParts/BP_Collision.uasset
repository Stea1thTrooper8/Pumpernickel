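; BP_Collision is a level part whose box destroys deletable balls that touch it and costs the player station health.
; On overlap, it checks the BP_Ball's CanBeDeleted flag, then clears that and the homing-return flag before destroying the ball.
; It then resets the ball count and decrements StationHP on the player's BP_Canon_Barrel pawn.
; Finally, it calls ReturnLightNormal on the BP_BaseRing found by class lookup.
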(event OnComponentBeginOverlap(BoxCol)
  (params (OverlappedComponent :type Primitive%20Component%20Object%20Reference) (OtherActor :type Actor%20Object%20Reference) (OtherComp :type Primitive%20Component%20Object%20Reference) (OtherBodyIndex :type Integer) (bFromSweep :type Boolean) (SweepResult :type Hit%20Result%20Structure%20%28by%20ref%29))
  (bind _asbp_ball (Utilities|Casting|CastToBP_Ball OtherActor))
  (if (Variables|/Game/Canon/BP_Ball.BP_Ball_C|GetCanBeDeleted _asbp_ball)
    (Variables|/Game/Canon/BP_Ball.BP_Ball_C|SetCanBeDeleted _asbp_ball false)
    (Variables|/Game/Canon/BP_Ball.BP_Ball_C|SetIsHomingReturn _asbp_ball false)
    (Actor|DestroyActor _asbp_ball)
    (bind _asbp_canon_barrel (Utilities|Casting|CastToBP_Canon_Barrel (Game|Player|GetPlayerPawn 0)))
    (Variables|/Game/Canon/BP_Canon_Barrel.BP_Canon_Barrel_C|SetBallCount _asbp_canon_barrel 0)
    (bind _output_get (Variables|/Game/Canon/BP_Canon_Barrel.BP_Canon_Barrel_C|SetStationHP _asbp_canon_barrel (- (stale _output_get) 1)))
    (bind _returnvalue (Actor|GetActorOfClass "/Game/LevelParts/BP_BaseRing.BP_BaseRing_C"))
    (Default|ReturnLightNormal _returnvalue)))

(fn ConstructionScript)