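; BP_BaseRing is a level-part ring that sets a BP_Ball's BounceCount to its MaxBounce on contact.
; Both actor overlap and Ring component hits run the same ball cast and assignment.
; The construction script creates a dynamic halo light material on the ring mesh.
; ReturnLightChange and ReturnLightNormal switch that halo's color between red and cyan, though nothing in this Blueprint calls them.
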(event OnComponentHit(Ring)
  (params (HitComponent :type Primitive%20Component%20Object%20Reference) (OtherActor :type Actor%20Object%20Reference) (OtherComp :type Primitive%20Component%20Object%20Reference) (NormalImpulse :type Vector :default "0, 0, 0") (Hit :type Hit%20Result%20Structure%20%28by%20ref%29))
  (bind _asbp_ball (Utilities|Casting|CastToBP_Ball OtherActor))
  (Variables|/Game/Canon/BP_Ball.BP_Ball_C|SetBounceCount _asbp_ball (Variables|/Game/Canon/BP_Ball.BP_Ball_C|GetMaxBounce _asbp_ball)))

(event EventBeginPlay)

(event Collision|EventActorBeginOverlap
  (params (OtherActor :type Actor%20Object%20Reference))
  (bind _asbp_ball (Utilities|Casting|CastToBP_Ball (stale OnComponentHit(Ring) OtherActor)))
  (Variables|/Game/Canon/BP_Ball.BP_Ball_C|SetBounceCount _asbp_ball (Variables|/Game/Canon/BP_Ball.BP_Ball_C|GetMaxBounce _asbp_ball)))

(fn ConstructionScript
  (bind _returnvalue (Rendering|Material|CreateDynamicMaterialInstance (Variables|Default|GetRing) 1 "/Game/Materials/M_halo_light.M_halo_light" "None" :!class /Script/Engine.PrimitiveComponent))
  (Variables|Default|SetReturnLight _returnvalue))

(fn ReturnLightChange
  (Rendering|Material|SetVectorParameterValue (Variables|Default|GetReturnLight) "HaloLight" "(R=1.000000,G=0.000000,B=0.000000,A=1.000000)" :!class /Script/Engine.MaterialInstanceDynamic))

(fn ReturnLightNormal
  (Rendering|Material|SetVectorParameterValue (Variables|Default|GetReturnLight) "HaloLight" "(R=0.141176,G=0.933333,B=1.000000,A=1.000000)" :!class /Script/Engine.MaterialInstanceDynamic))